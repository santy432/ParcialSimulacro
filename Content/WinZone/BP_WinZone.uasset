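; BP_WinZone is a trigger actor that wins the game when the player reaches it with every relic.
; On BeginPlay it caches the GS_GameState and GM_MyGameMode references.
; When BP_FirstPersonCharacter begins overlapping it, it checks the game state's HasAllReliq flag and, if set, calls WinGame on the game mode.
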(event EventBeginPlay
  (bind _asgs_game_state (Utilities|Casting|CastToGS_GameState (Game|GetGameState)))
  (Variables|Default|SetAs%20GS%20Game%20State _asgs_game_state)
  (bind _asgm_my_game_mode (Utilities|Casting|CastToGM_MyGameMode (Game|GetGameMode)))
  (Variables|Default|SetAs%20GM%20My%20Game%20Mode _asgm_my_game_mode))

(event Collision|EventActorBeginOverlap
  (params (OtherActor :type Actor%20Object%20Reference))
  (Utilities|Casting|CastToBP_FirstPersonCharacter OtherActor)
  (if (Variables|/Game/Base/GS_GameState.GS_GameState_C|GetHasAllReliq (Variables|Default|GetAs%20GS%20Game%20State))
    (Default|WinGame (Variables|Default|GetAs%20GM%20My%20Game%20Mode))))

(event EventTick
  (params (DeltaSeconds :type Float%20%28single-precision%29)))

(fn ConstructionScript)