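; BP_Platform is a moving platform that activates when the first-person character hits it while GS_GameState reports all "Reliq" collected.
; A DoOnce lets that hit start the motion a single time.
; A timeline lerps the Cube's world location between the Bottom and Top components.
; On finish it re-calls StartPlatform, where a FlipFlop alternates forward and reverse playback for an endless back-and-forth.
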(event Custom|StartPlatform
  (Utilities|FlowControl|FlipFlop
    (:A
      (bind _newtrack_0 (Timeline|Timeline PlayFromStart)
        (:Update
          (Transformation|SetWorldLocation (Variables|Default|GetCube) (Math|Vector|Lerp(Vector) (Transformation|GetWorldLocation (Variables|Default|GetBottom)) (Transformation|GetWorldLocation (Variables|Default|GetTop)) _newtrack_0) false false))
        (:Finished
          (CallFunction|StartPlatform))))
    (:B
      (Timeline|Timeline ReverseFromEnd))))

(event EventBeginPlay
  (bind _asgs_game_state (Utilities|Casting|CastToGS_GameState (Game|GetGameState)))
  (Variables|Default|SetAs%20GS%20Game%20State _asgs_game_state))

(event Collision|EventHit
  (params (MyComp :type Primitive%20Component%20Object%20Reference) (Other :type Actor%20Object%20Reference) (OtherComp :type Primitive%20Component%20Object%20Reference) (bSelfMoved :type Boolean) (HitLocation :type Vector :default "0, 0, 0") (HitNormal :type Vector :default "0, 0, 0") (NormalImpulse :type Vector :default "0, 0, 0") (Hit :type Hit%20Result%20Structure%20%28by%20ref%29))
  (Utilities|Casting|CastToBP_FirstPersonCharacter Other)
  (if (Variables|/Game/Base/GS_GameState.GS_GameState_C|GetHasAllReliq (Variables|Default|GetAs%20GS%20Game%20State))
    (Utilities|FlowControl|DoOnce false
      (:Completed
        (CallFunction|StartPlatform)))))

(fn ConstructionScript)