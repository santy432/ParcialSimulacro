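; GM_MyGameMode is a game mode that runs a timed win-or-lose match and owns the HUD.
; BeginPlay creates the WB_HUD widget and adds it to the viewport.
; Tick counts TimeLeft down until the match ends, showing the lose screen when it runs out.
; WinGame shows the win screen and sets HasEnded, which also stops the countdown.
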(event EventBeginPlay
  (bind _returnvalue (UserInterface|CreateWidget "/Game/Ui/WB_HUD.WB_HUD_C"))
  (bind _output_get (Variables|Default|SetHUD _returnvalue))
  (UserInterface|Viewport|AddtoViewport _output_get 0))

(event EventTick
  (params (DeltaSeconds :type Float%20%28single-precision%29))
  (if (not (Variables|Default|GetHasEnded))
    (bind _output_get (Variables|Default|SetTimeLeft (- (Variables|Default|GetTimeLeft) DeltaSeconds)))
    (if (<= _output_get 0.0)
      (Default|SetLoseScreen (Variables|Default|GetHUD))
      (Variables|Default|SetTimeLeft 0.0)
      (Variables|Default|SetHasEnded true))))

(fn ConstructionScript)

(fn WinGame
  (Default|SetWinScreen (Variables|Default|GetHUD))
  (Variables|Default|SetHasEnded true))