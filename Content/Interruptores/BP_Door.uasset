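; BP_Door is a door that removes itself once enough switch interactions have occurred.
; On BeginPlay it binds a handler to the interaction event of every switch in its Interruptores array.
; Each event increments a counter, and the door destroys itself when the count reaches the number of switches.
; The counter does not track which switch fired, so any repeated events also count toward the total.
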(event Custom|OnInterruptorInteract
  (bind _output_get (Variables|Default|SetInterruptoresActivos (+ (Variables|Default|GetInterruptoresActivos) 1)))
  (if (>= _output_get (Utilities|Array|Length (Variables|Default|GetInterruptores)))
    (Actor|DestroyActor)))

(event EventBeginPlay
  (for _array_element (Variables|Default|GetInterruptores)
    (EventDispatchers|BindEventtoOnInteraction _array_element (delegate Custom|OnInterruptorInteract))))

(fn ConstructionScript)